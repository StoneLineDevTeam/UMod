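; SplinePath is an actor Blueprint that moves a referenced ActorToMove along its Path spline in a continuous loop.
; Each tick adds Speed to the travelled distance without delta-time scaling, so movement is frame-rate dependent, and resets it to zero at the spline's end.
; BeginPlay and Tick share the placement step, which snaps location to the spline and eases rotation toward its direction with a fixed-alpha lerp.
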(event EventBeginPlay
  (bind _path (Variables|Default|GetPath))
  (bind _distancealongspline (Variables|Default|GetDistanceAlongSpline))
  (bind _actortomove (Variables|Default|GetActorToMove))
  (Transformation|SetActorLocation _actortomove (Spline|GetLocationatDistanceAlongSpline _path _distancealongspline "World") false false)
  (Transformation|SetActorRotation _actortomove (Math|Rotator|Lerp(Rotator) (Transformation|GetActorRotation _actortomove) (Spline|GetRotationatDistanceAlongSpline _path _distancealongspline "World") 0.05 true)))

(event EventTick
  (params (DeltaSeconds :type Float%20%28single-precision%29))
  (bind _path (Variables|Default|GetPath))
  (bind _actortomove (Variables|Default|GetActorToMove))
  (if (>= (Variables|Default|GetDistanceAlongSpline) (Spline|GetSplineLength _path))
    (Variables|Default|SetDistanceAlongSpline 0.0)
    (else
      (Variables|Default|SetDistanceAlongSpline (+ (Variables|Default|GetDistanceAlongSpline) (Variables|Default|GetSpeed)))
      (Transformation|SetActorLocation _actortomove (Spline|GetLocationatDistanceAlongSpline _path (Variables|Default|GetDistanceAlongSpline) "World") false false)
      (Transformation|SetActorRotation _actortomove (Math|Rotator|Lerp(Rotator) (Transformation|GetActorRotation _actortomove) (Spline|GetRotationatDistanceAlongSpline _path (Variables|Default|GetDistanceAlongSpline) "World") 0.05 true)))))

(fn ConstructionScript)